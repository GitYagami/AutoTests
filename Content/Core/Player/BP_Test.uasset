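; BP_Test is a functional test that checks the player's left machine gun trace and path movement.
; PrepareTest caches the player pawn as BP_Player along with its BPPath.
; StartTest fires the weapon component's left machine gun line trace from the player camera with persistent debug drawing.
; It succeeds only if the hit actor is tagged Destructible while the path's Move is playing, and fails otherwise.
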(event `self.ReceivePrepareTest`
  (bind _asbp_player (cast `/Game/Core/Player/BP_Player` (`GameplayStatics.GetPlayerPawn` 0)))
  (bind _output_get (set `self.BP_Player` _asbp_player))
  (set `self.BP Path` (`/Game/Core/Player/BP_Player.BP_Path` _output_get)))

(event `self.ReceiveStartTest`
  (bind _bp_player (`self.BP_Player`))
  (bind _outhit (`/Game/Core/Weapons/BP_WeaponComponent.ShootLeft_MachineGun_LineTrace` (`/Game/Core/Player/BP_Player.BP_WeaponComponent` _bp_player) (`/Game/Core/Player/BP_Player.Camera` _bp_player) _bp_player 0.0 "Persistent" 200.0))
  (if (and (`self.ActorHasTag` (`.HitActor` (`GameplayStatics.BreakHitResult` _outhit)) "Destructible") (`TimelineComponent.IsPlaying` (`/Game/Core/Player/BP_Path.Move` (`self.BP Path`))))
    (`self.FinishTest` "Succeeded" "On a touché un Destructible \nET \nOn avance bien")
    (else
      (`self.FinishTest` "Failed" "FAIL TEST"))))

(fn `UserConstructionScript`)