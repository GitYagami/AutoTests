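; Pooled projectile for the player's right weapon, launched along the camera's forward vector when taken into use.
; HoldMultiplicator scales its launch speed and the masterfield scale, radial magnitude and directional magnitude from RightWeaponValues.
; The sphere's first hit reports impact location, normal, hit actor and those scaled values to the player's BP_WeaponComponent.
; Releasing it to the pool zeroes velocity and resets the DoOnce, so the reused actor can report again.
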(event `self.Sphere.OnComponentHit`
  (params (HitComponent :type "PrimitiveComponent Object Reference") (OtherActor :type "Actor Object Reference") (OtherComp :type "PrimitiveComponent Object Reference") (NormalImpulse :type "Vector Structure") (Hit :type "HitResult Structure (by ref)"))
  (bind _holdmultiplicator (`self.HoldMultiplicator`))
  (bind ((`RightWeaponMasterfieldScale_6_5F9027A04CC98077B7FDACBC614CFF94` _rightweaponmasterfieldscale) (`RightWeaponRadialMagnitude_9_76AEE13A4B5D08D02AFFF1B01C046926` _rightweaponradialmagnitude) (`RightWeaponDirectionalMagnitude_11_AA1A509D4F2FAE2F07B539A850D748C5` _rightweapondirectionalmagnitude)) (break `/Game/Core/Player/RightWeaponValues` (`self.RightWeaponValues`)))
  ;[0.15 0.15 0.15 0.5 40] COLLISION SPHERE (peut être changé en overlap si besoin, juste changer les collisions de la sphere)
  (`/Engine/EditorBlueprintResources/StandardMacros.DoOnce` false :!pinned true :!label _label ; Obligé de connecter le reste car avec le PoolComponent, ce code ne se fait qu'une seule fois sinon. Etant donné qu'on réutilise le même BP
    (:`Completed`
      (message `/Game/Core/Interfaces/BPI_ToWeaponComponent.ProjectileHitSomething` (`self.GetComponentByClass` (`GameplayStatics.GetPlayerPawn` 0) "/Game/Core/Weapons/BP_WeaponComponent.BP_WeaponComponent_C") Hit_Location Hit_ImpactNormal (* _rightweaponmasterfieldscale _holdmultiplicator) (* _rightweaponradialmagnitude _holdmultiplicator) (* _rightweapondirectionalmagnitude _holdmultiplicator) OtherActor))))

(event `self.SetInUse`
  (params (InUse :type Boolean))
  ;[0.15 0.15 0.15 0.5 40] ObjectPool
  (`parent.SetInUse` InUse)
  (if InUse
    (`self.SetProjectileValues` (`.RightWeaponVelocity_3_DF93187B48B1403037B0B4A2324B6899` (break `/Game/Core/Player/RightWeaponValues` (`self.RightWeaponValues`))))
    (else
      (set `MovementComponent.Velocity` (0.0 0.0 0.0) (`self.ProjectileMovement`))
      (goto _label :!via `Reset`))))

(fn `SetProjectileValues`
  (params (ProjectileVelocity :type "Float (single-precision)"))
  (bind (_returnvalue_x _returnvalue_y _returnvalue_z) (`KismetMathLibrary.BreakVector` (* (`self.GetActorForwardVector` (`GameplayStatics.GetPlayerCameraManager` 0)) (* ProjectileVelocity (`self.HoldMultiplicator`)))))
  (set `MovementComponent.Velocity` (`KismetMathLibrary.MakeVector` _returnvalue_x _returnvalue_y _returnvalue_z) (`self.ProjectileMovement`)))

(fn `UserConstructionScript`)